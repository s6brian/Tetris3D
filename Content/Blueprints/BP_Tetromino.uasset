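; BP_Tetromino defines the seven standard tetromino shapes (I, J, L, S, Z, T, O) for a Tetris-style game.
; Its construction script converts each shape's bitmap variable into a matrix with MakeTetrominoMatrix and passes the array to InitiateTetrominoShapes.
; Graph comments note that the bitmaps are flat 0/1 sequences read left to right, bottom to top.
; The event graph holds only disabled placeholder events.
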(event EventBeginPlay)

(event Collision|EventActorBeginOverlap
  (params (OtherActor :type Actor%20Object%20Reference)))

(event EventTick
  (params (DeltaSeconds :type Float%20%28single-precision%29)))

(fn ConstructionScript
  (Class|Tetromino|InitiateTetrominoShapes (Utilities|Array|MakeArray (Utilities|Struct|MakeTetrominoMatrix (Variables|Default|GetTetrominoBitMapI)) (Utilities|Struct|MakeTetrominoMatrix (Variables|Default|GetTetrominoBitMapJ)) (Utilities|Struct|MakeTetrominoMatrix (Variables|Default|GetTetrominoBitMapL)) (Utilities|Struct|MakeTetrominoMatrix (Variables|Default|GetTetrominoBitMapS)) (Utilities|Struct|MakeTetrominoMatrix (Variables|Default|GetTetrominoBitMapZ)) (Utilities|Struct|MakeTetrominoMatrix (Variables|Default|GetTetrominoBitMapT)) (Utilities|Struct|MakeTetrominoMatrix (Variables|Default|GetTetrominoBitMapO)))))